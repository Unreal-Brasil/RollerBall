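; Game mode that ends the player's run when their score falls behind elapsed time.
; BeginPlay caches the BP_TheHeroInstance game instance, which holds PlayerScore and PlayerTime.
; Tick compares the two once PlayerTime passes a short grace threshold, and a score below the time triggers CallPlayerDied through a DoOnce so it fires only once.
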(event EventBeginPlay
  (bind _asbp_the_hero_instance (Utilities|Casting|CastToBP_TheHeroInstance (Game|GetGameInstance)))
  (Variables|Default|SetTheHeroInstance _asbp_the_hero_instance))

(event EventTick
  (params (DeltaSeconds :type Float%20%28single-precision%29))
  (bind _theheroinstance (Variables|Default|GetTheHeroInstance))
  (bind _playertime (Variables|/Script/TheHero.TheHeroInstance|GetPlayerTime _theheroinstance))
  (Utilities|IsValid _theheroinstance
    (:Is%20Valid
      (if (> _playertime 10)
        (if (< (Variables|/Script/TheHero.TheHeroInstance|GetPlayerScore _theheroinstance) _playertime)
          (Utilities|FlowControl|DoOnce false
            (:Completed
              (Default|CallPlayerDied))))))))

(fn ConstructionScript)