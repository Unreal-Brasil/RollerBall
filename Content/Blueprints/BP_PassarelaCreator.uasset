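; Procedural walkway spawner for a rolling-ball game, stacking random Passarelas meshes at AlturaPlataformas intervals along Z.
; The first mesh is built at construction; a batch follows at BeginPlay, then a looping timer adds more.
; Each spawn moves the death box and arrow to the newest level and adds a one-shot trigger that awards score, particles and sound.
; Another timer destroys mesh components above the player.
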(event OnComponentBeginOverlap(BoxDeath)
  (params (OverlappedComponent :type Primitive%20Component%20Object%20Reference) (OtherActor :type Actor%20Object%20Reference) (OtherComp :type Primitive%20Component%20Object%20Reference) (OtherBodyIndex :type Integer) (bFromSweep :type Boolean) (SweepResult :type Hit%20Result%20Structure%20%28by%20ref%29))
  (Utilities|Casting|CastToTP_RollingBallPlayer OtherActor)
  (Default|CallPlayerDied))

(event Custom|LOAD_PLATFORM
  (Variables|Default|SetCounter (+ (Variables|Default|GetCounter) 1))
  (Utilities|FlowControl|Sequence
    (:then_0
      (bind _returnvalue (AddComponent|AddStaticMeshComponent false (Math|Transform|MakeTransform (Math|Vector|MakeVector 0.0 0.0 (* (Variables|Default|GetCounter) (Variables|Default|GetAlturaPlataformas))) "0, 0, 0" "3.000000,1,1")))
      (Components|StaticMesh|SetStaticMesh _returnvalue (Utilities|Array|Get(acopy) (Variables|Default|GetPassarelas) (Math|Random|RandomIntegerinRange 1 (- (Utilities|Array|Length (Variables|Default|GetPassarelas)) 1)))))
    (:then_1
      (Transformation|SetRelativeLocation (Variables|Default|GetArrowDOWN) (Math|Vector|MakeVector 0.0 0.0 (* (Variables|Default|GetCounter) (Variables|Default|GetAlturaPlataformas))) false false))
    (:then_2
      (Transformation|SetRelativeLocation (Variables|Default|GetBoxDeath) (Math|Vector|MakeVector 0.0 0.0 (* (Variables|Default|GetCounter) (Variables|Default|GetAlturaPlataformas))) false false))
    (:then_3
      (bind _returnvalue_2 (AddComponent|AddBoxComponent false (Math|Transform|MakeTransform (Math|Vector|MakeVector 0.0 0.0 (* (Variables|Default|GetCounter) (Variables|Default|GetAlturaPlataformas))) "0, 0, 0" "4.000000,42.000000,2.000000")))
      (Collision|AssignOnComponentBeginOverlap _returnvalue_2 (delegate Custom|OnComponentBeginOverlap_Event_0)))))

(event Custom|OnComponentBeginOverlap_Event_0
  (params (OverlappedComponent :type Primitive%20Component%20Object%20Reference) (OtherActor :type Actor%20Object%20Reference) (OtherComp :type Primitive%20Component%20Object%20Reference) (OtherBodyIndex :type Integer) (bFromSweep :type Boolean) (SweepResult :type Hit%20Result%20Structure%20%28by%20ref%29))
  (bind _pointtodelivery (Variables|Default|GetPointToDelivery))
  (Components|DestroyComponent OverlappedComponent)
  (bind _astp_rolling_ball_player (Utilities|Casting|CastToTP_RollingBallPlayer OtherActor))
  (Default|ShowParticle _astp_rolling_ball_player)
  (Default|CallPlayerGotPoint _pointtodelivery)
  (bind _asbp_the_hero_instance (Utilities|Casting|CastToBP_TheHeroInstance (Game|GetGameInstance)))
  (Class|TheHeroInstance|UpdatePlayerScore _asbp_the_hero_instance _pointtodelivery)
  (Audio|Components|Audio|Play (Variables|Default|GetAudio) 0.0))

(event Custom|EvtDestroyPlatform
  (for _array_element (Actor|GetComponentsByClass "/Script/Engine.StaticMeshComponent")
    (bind _astp_rolling_ball_player (Utilities|Casting|CastToTP_RollingBallPlayer (Game|Player|GetPlayerPawn 0)))
    (if (> (.z (Transformation|GetWorldLocation _array_element)) (.z (Transformation|GetActorLocation _astp_rolling_ball_player)))
      (Components|DestroyComponent _array_element))))

(event EventBeginPlay
  (Utilities|FlowControl|Sequence
    (:then_0
      (Utilities|Time|SetTimerbyEvent (delegate Custom|LOAD_PLATFORM) 3.0 true))
    (:then_1
      (for _index (range 0 4)
        (Variables|Default|SetCounter (+ (Variables|Default|GetCounter) 1))
        (Utilities|FlowControl|Sequence
          (:then_0
            (bind _returnvalue (AddComponent|AddStaticMeshComponent false (Math|Transform|MakeTransform (Math|Vector|MakeVector 0.0 0.0 (* (Variables|Default|GetCounter) (Variables|Default|GetAlturaPlataformas))) "0, 0, 0" "3.000000,1,1")))
            (Components|StaticMesh|SetStaticMesh _returnvalue (Utilities|Array|Get(acopy) (Variables|Default|GetPassarelas) (Math|Random|RandomIntegerinRange 1 (- (Utilities|Array|Length (Variables|Default|GetPassarelas)) 1)))))
          (:then_1
            (Transformation|SetRelativeLocation (Variables|Default|GetArrowDOWN) (Math|Vector|MakeVector 0.0 0.0 (* (Variables|Default|GetCounter) (Variables|Default|GetAlturaPlataformas))) false false))
          (:then_2
            (Transformation|SetRelativeLocation (Variables|Default|GetBoxDeath) (Math|Vector|MakeVector 0.0 0.0 (* (Variables|Default|GetCounter) (Variables|Default|GetAlturaPlataformas))) false false))
          (:then_3
            (bind _returnvalue_2 (AddComponent|AddBoxComponent false (Math|Transform|MakeTransform (Math|Vector|MakeVector 0.0 0.0 (* (Variables|Default|GetCounter) (Variables|Default|GetAlturaPlataformas))) "0, 0, 0" "4.000000,42.000000,2.000000")))
            (Collision|AssignOnComponentBeginOverlap _returnvalue_2 (delegate Custom|OnComponentBeginOverlap_Event_0))))))
    (:then_2
      (Utilities|Time|SetTimerbyEvent (delegate Custom|EvtDestroyPlatform) 5.0 true))))

(fn ConstructionScript
  (Utilities|FlowControl|Sequence
    (:then_0
      (bind _returnvalue (AddComponent|AddStaticMeshComponent false (Math|Transform|MakeTransform (Math|Vector|MakeVector 0.0 0.0 (* 0 (Variables|Default|GetAlturaPlataformas))) "0, 0, 0" "3.000000,1,1")))
      (Components|StaticMesh|SetStaticMesh _returnvalue (Utilities|Array|Get(acopy) (Variables|Default|GetPassarelas))))))